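; Shared health component that binds to its owner's damage event, tracks current health and broadcasts damage taken and death.
; Damage accumulates into a pending amount that a self-calling Delay loop drains from health in small steps.
; Death is checked only on each hit, right after the drain starts, not when it finishes.
; A similar regeneration loop exists but is not called here, and Tick prints health for debugging.
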(event Custom|OnTakeAnyDamage
  (params (DamagedActor :type Actor%20Object%20Reference) (Damage :type Float%20%28single-precision%29) (DamageType :type Damage%20Type%20Object%20Reference) (InstigatedBy :type Controller%20Object%20Reference) (DamageCauser :type Actor%20Object%20Reference))
  (Variables|Default|SetEnemyDamage (+ Damage (Variables|Default|GetEnemyDamage)))
  (if (> Damage 0.0)
    (Variables|Default|SetShouldDrain? true)
    (CallFunction|DepreciateHealth)
    (Default|CallOnDamageTaken)
    (if (CallFunction|IsDead)
      (Default|CallOnDeath))))

(event Custom|DepreciateHealth
  (if (Variables|Default|GetShouldDrain?)
    (if (<= (Math|Float|Clamp(Float) (- (Variables|Default|GetCurrentHealth) (Variables|Default|GetHealthReductionSpeed)) 0.0 (Variables|Default|GetMaxHealth)) 0.0)
      (Variables|Default|SetCurrentHealth 0.0)
      (else
        (Variables|Default|SetCurrentHealth (Math|Float|Clamp(Float) (- (Variables|Default|GetCurrentHealth) (Variables|Default|GetHealthReductionSpeed)) 0.0 (Variables|Default|GetMaxHealth)))
        (bind _output_get (Variables|Default|SetEnemyDamage (Math|Float|Clamp(Float) (- (Variables|Default|GetEnemyDamage) (Variables|Default|GetHealthReductionSpeed)) 0.0 (Variables|Default|GetMaxHealth))))
        (if (<= _output_get 0.0)
          (Variables|Default|SetShouldDrain? false)
          (Variables|Default|SetEnemyDamage 0.0)
          (else
            (Utilities|FlowControl|Delay 0.001)
            (CallFunction|DepreciateHealth)))))))

(event Custom|AppreciateHealth
  (if (not (CallFunction|IsDead))
    (if (not (Variables|Default|GetShouldDrain?))
      (if (not (== (Variables|Default|GetCurrentHealth) (Variables|Default|GetMaxHealth)))
        (Variables|Default|SetCurrentHealth (Math|Float|Clamp(Float) (+ (Variables|Default|GetCurrentHealth) 0.1) 0.0 (Variables|Default|GetMaxHealth)))
        (Utilities|FlowControl|Delay 0.08)
        (CallFunction|AppreciateHealth)))))

(event EventBeginPlay
  (Variables|Default|SetCurrentHealth (Variables|Default|GetMaxHealth))
  (EventDispatchers|AssignOnTakeAnyDamage (Components|GetOwner) (delegate Custom|OnTakeAnyDamage)))

(event EventTick
  (params (DeltaSeconds :type Float%20%28single-precision%29))
  (Development|PrintString (Utilities|String|ToString(Float) (Variables|Default|GetCurrentHealth))))

(fn IsDead
  (return (<= (Variables|Default|GetCurrentHealth) 0.0)))