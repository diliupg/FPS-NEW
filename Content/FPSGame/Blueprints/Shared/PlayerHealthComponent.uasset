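; Player health component that tracks current and previous health, subtracting damage received through the owner's any-damage event.
; It broadcasts OnDamageTaken before health is reduced and OnDeath when health reaches zero or below.
; DrainHealth and RegenHealth step health in small increments through self-calling Delay loops, with ShouldDrain gating which runs.
; Draining stops at zero without broadcasting death, and regeneration climbs more slowly toward MaxHealth.
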(event Custom|OnTakeAnyDamage
  (params (DamagedActor :type Actor%20Object%20Reference) (Damage :type Float%20%28single-precision%29) (DamageType :type Damage%20Type%20Object%20Reference) (InstigatedBy :type Controller%20Object%20Reference) (DamageCauser :type Actor%20Object%20Reference))
  (if (> Damage 0.0)
    ;[0.01381 0.1283 0.5] set previous health before we reduce current health
    (Variables|Default|SetPreviousHealth (Variables|Default|GetCurrentHealth))
    (Default|CallOnDamageTaken)
    (Variables|Default|SetCurrentHealth (- (Variables|Default|GetCurrentHealth) Damage))
    (if (CallFunction|IsDead)
      (Default|CallOnDeath))))

(event Custom|DrainHealth
  (if (Variables|Default|GetShouldDrain?)
    (bind _output_get (Variables|Default|SetCurrentHealth (Math|Float|Clamp(Float) (- (Variables|Default|GetCurrentHealth) 0.1) 0.0 (Variables|Default|GetMaxHealth))))
    (if (== _output_get 0.0)
      (Variables|Default|SetShouldDrain? false)
      (else
        (Utilities|FlowControl|Delay 0.005)
        (CallFunction|DrainHealth)))))

(event Custom|RegenHealth
  (if (not (Variables|Default|GetShouldDrain?))
    (if (not (== (Variables|Default|GetCurrentHealth) (Variables|Default|GetMaxHealth)))
      (Variables|Default|SetCurrentHealth (Math|Float|Clamp(Float) (+ (Variables|Default|GetCurrentHealth) 0.1) 0.0 (Variables|Default|GetMaxHealth)))
      (Utilities|FlowControl|Delay 0.08)
      (CallFunction|RegenHealth))))

(event EventBeginPlay
  (bind _output_get (Variables|Default|SetCurrentHealth (Variables|Default|GetMaxHealth)))
  (Variables|Default|SetPreviousHealth _output_get)
  (EventDispatchers|AssignOnTakeAnyDamage (Components|GetOwner) (delegate Custom|OnTakeAnyDamage)))

(fn IsDead
  (return (<= (Variables|Default|GetCurrentHealth) 0.0)))