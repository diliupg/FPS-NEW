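; Anim notify state for a left-arm melee attack that damages actors tagged Player.
; Each notify tick runs a sphere trace for Pawn objects from the left elbow socket to the left fingertip socket, with timed debug drawing.
; A hit on a tagged actor applies fixed damage, with no guard against repeat hits on later ticks.
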(fn ReceivedNotifyTick
  (params (MeshComp :type Skeletal%20Mesh%20Component%20Object%20Reference) (Animation :type Anim%20Sequence%20Base%20Object%20Reference) (FrameDeltaTime :type Float%20%28single-precision%29))
  (bind (_outhit _returnvalue) (Collision|SphereTraceForObjects MeshComp (Transformation|GetSocketLocation MeshComp "LeftElbowSocket") (Transformation|GetSocketLocation MeshComp "LeftFingertipSocket") 2e+01 (Utilities|Array|MakeArray "ObjectTypeQuery3") false (Utilities|Array|MakeArray 0) "ForDuration" true "(R=1.000000,G=0.000000,B=0.000000,A=1.000000)" "(R=0.000000,G=1.000000,B=0.000000,A=1.000000)" 2.0))
  (if _returnvalue
    (if (Actor|ActorHasTag (.HitActor (Collision|BreakHitResult _outhit)) "Player")
      (Game|Damage|ApplyDamage (.HitActor (Collision|BreakHitResult _outhit)) 1e+01 0 0 "/Script/Engine.DamageType")
      (return false))))