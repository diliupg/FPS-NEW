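; PlayerHealthComponent is a player health component, marked unused, meant to track damage and death.
; Its damage handler accumulates pending damage, calls DepreciateHealth and fires damage and death dispatchers.
; The drain and regeneration events are empty; their delayed recursive logic for gradual health change is disconnected.
; Health initialization and binding to the owner's damage event are also disconnected, leaving BeginPlay empty.
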(event Custom|OnTakeAnyDamage
  (params (DamagedActor :type Actor%20Object%20Reference) (Damage :type Float%20%28single-precision%29) (DamageType :type Damage%20Type%20Object%20Reference) (InstigatedBy :type Controller%20Object%20Reference) (DamageCauser :type Actor%20Object%20Reference))
  ;[1 0 0.01469] PLAYER HEALTH COMPONENT IS UNUSED!
  (Variables|Default|SetEnemyDamage (+ Damage (Variables|Default|GetEnemyDamage)))
  (if (> Damage 0.0)
    (Variables|Default|SetShouldDrain? true)
    (CallFunction|DepreciateHealth)
    (Default|CallOnDamageTakenD)
    (if (CallFunction|IsDead)
      (Default|CallOnDeathD))))

(event Custom|DepreciateHealth
  ;[1 0 0.01469] PLAYER HEALTH COMPONENT IS UNUSED!
  ;;[0.5 0.01161 0.07146] Depreciate Health
)

(event Custom|AppreciateHealth
  ;[1 0 0.01469] PLAYER HEALTH COMPONENT IS UNUSED!
  ;;[0 0.5 0.01933] Appreciate Health, if player is alive.
)

(event EventBeginPlay
  ;[1 0 0.01469] PLAYER HEALTH COMPONENT IS UNUSED!
)

(fn IsDead
  (return (<= (Variables|Default|GetCurrentHealth) 0.0)))