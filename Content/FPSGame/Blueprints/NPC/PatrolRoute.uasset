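; PatrolRoute is an NPC patrol route Blueprint that supplies world-space waypoints from the points of its PatrolPath spline.
; GetNextPointAsWorldPosition returns the spline point at the current PatrolIndex.
; The IncreasePatrolPath event advances that index with a modulo wrap, so the route loops, and the index lives on the route itself.
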(event Custom|IncreasePatrolPath
  (Variables|Default|SetPatrolIndex (Math|Integer|%(Integer) (+ (Variables|Default|GetPatrolIndex) 1) (Spline|GetNumberOfSplinePoints (Variables|Default|GetPatrolPath)))))

(event EventBeginPlay)

(event Collision|EventActorBeginOverlap
  (params (OtherActor :type Actor%20Object%20Reference)))

(event EventTick
  (params (DeltaSeconds :type Float%20%28single-precision%29)))

(fn ConstructionScript)

(fn GetNextPointasWorldPosition
  (return (Spline|GetLocationatSplinePoint (Variables|Default|GetPatrolPath) (Variables|Default|GetPatrolIndex) "World")))