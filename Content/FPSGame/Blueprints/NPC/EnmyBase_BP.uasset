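; Base enemy character that detects and chases the player and provides sword combat actions.
; BeginPlay starts a delayed, self-recalling box trace forward from the head socket, moving the AI toward any BP_Player hit.
; Separate events spawn a sword onto a hand socket and play an attack montage that signals its end.
; Helper functions expose the patrol route and map movement states to walk speeds.
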(event Custom|LookForLight
  (bind _mesh (Variables|Character|GetMesh))
  (bind _returnvalue (Transformation|GetSocketLocation _mesh "HeadSocket"))
  (Utilities|FlowControl|Delay 0.5)
  (bind (_outhit _returnvalue_2) (Collision|BoxTraceByChannel _returnvalue (+ _returnvalue (* (Math|Vector|GetForwardVector (Transformation|GetActorRotation)) 7e+02)) "70.000000,70.000000,50.000000" "0, 0, 0" "TraceTypeQuery1" false 0 "None" true "(R=1.000000,G=0.000000,B=0.000000,A=1.000000)" "(R=0.000000,G=1.000000,B=0.000000,A=1.000000)" 1.0))
  (if _returnvalue_2
    (Utilities|Casting|CastToBP_Player (.HitActor (Collision|BreakHitResult _outhit))
      (:then
        (AI|AIMoveTo self (Transformation|GetWorldLocation (.HitComponent (Collision|BreakHitResult _outhit))) 0 5.0 false
          (:OnSuccess
            _)))
      (:CastFailed
        _)))
  (CallFunction|LookforLight))

(event Custom|WeldSword
  (bind _returnvalue (Game|SpawnActorfromClass "/Game/FPSGame/Blueprints/EnemyWeapons/BP_Sword.BP_Sword_C" (Transformation|GetActorTransform) "Undefined" 0 0))
  (Transformation|AttachComponentToComponent _returnvalue (Variables|Character|GetMesh) "SwordSocket" "SnapToTarget" "SnapToTarget" "SnapToTarget" true)
  (Variables|Default|SetIsWeildingSword true))

(event Custom|AttackPlayer
  (Animation|Montage|PlayMontage (Variables|Character|GetMesh) "/Game/FPSGame/NPC/Characters/EnemyBase/Animations/Sowrd_Attack_Combo_CL_Heavy_Montage.Sowrd_Attack_Combo_CL_Heavy_Montage"
    (:OnCompleted
      _)
    (:OnInterrupted
      _))
  (Default|CallOnAttackEnd) ; event dispatched only when animation is completed or interrupted.
)

(event EventBeginPlay
  (CallFunction|LookforLight))

(fn ConstructionScript)

(fn GetPatrolRoute
  (return (Variables|Default|GetPatrolRoute)))

(fn SetMovementSpeed
  (params (Speed :type E_MovementSpeed%20Enum :default "NewEnumerator0"))
  (bind _output_get (Variables|/Script/Engine.CharacterMovementComponent|SetMaxWalkSpeed (Variables|Character|GetCharacterMovement) (Utilities|Select :Index Speed :NewEnumerator0 0.0 :NewEnumerator1 2e+02 :NewEnumerator2 3e+02 :NewEnumerator3 5e+02)))
  (return _output_get))