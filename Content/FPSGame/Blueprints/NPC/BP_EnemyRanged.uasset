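; BP_EnemyRanged is a ranged enemy NPC that arms itself with a rifle when play begins.
; BeginPlay calls EquipWeapon, which spawns BP_WeaponRifle, snaps it to the mesh's RifleSocket, sets the wielding flag and fires OnWeaponEquipped.
; The parent BeginPlay call is left unwired, so inherited BeginPlay logic does not run; the construction script only calls its parent.
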(event EventBeginPlay
  (CallFunction|EquipWeapon))

(event Collision|EventActorBeginOverlap
  (params (OtherActor :type Actor%20Object%20Reference)))

(event EventTick
  (params (DeltaSeconds :type Float%20%28single-precision%29)))

(event EventEquipWeapon
  (bind _returnvalue (Game|SpawnActorfromClass "/Game/FPSGame/Blueprints/EnemyWeapons/BP_WeaponRifle.BP_WeaponRifle_C" (Math|Transform|MakeTransform "0, 0, 0") "Undefined" 0 0))
  (bind _output_get (Variables|Default|SetWeaponActor _returnvalue))
  (Transformation|AttachComponentToComponent _output_get (Variables|Character|GetMesh) "RifleSocket" "SnapToTarget" "SnapToTarget" "SnapToTarget" true)
  (Variables|Default|SetIsWeildingweapon true)
  (Default|CallOnWeaponEquipped))

(fn ConstructionScript
  (|CallParentFunction))