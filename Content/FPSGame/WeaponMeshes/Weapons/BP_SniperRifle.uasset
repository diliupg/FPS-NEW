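; Sniper rifle weapon Blueprint that extends a parent weapon class with a firing animation and a scoped aim view.
; Shooting runs the parent logic, plays the rifle's fire animation on the weapon mesh, then calls the fire rate calculation.
; Entering aim as the current weapon adds a SniperScope widget and hides the weapon mesh, player character and main HUD.
; Exiting aim removes the scope and shows all three again.
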(event EventWeaponAimEnter
  (|CallParentFunction)
  (if (== (Variables|/Game/FPSGame/_PlayerCharacter/BP_Player.BP_Player_C|GetCurrentWeapon (Variables|Default|GetPlayer)) self)
    (bind _returnvalue (UserInterface|CreateWidget "/Game/FPSGame/UI/SniperScope.SniperScope_C"))
    (if (not (UserInterface|Viewport|IsinViewport _returnvalue))
      (UserInterface|Viewport|AddtoViewport _returnvalue 0)
      ;[0 0.02795 0.2656] Hides weapon, player and HUD while aiming sniper rifle
      (Development|SetHiddeninGame (Variables|Default|GetWeaponMesh) true false)
      (Rendering|SetActorHiddenInGame (Game|GetPlayerCharacter 0) true)
      (Widget|SetVisibility (Variables|/Game/FPSGame/_PlayerCharacter/BP_Player.BP_Player_C|GetMainHUD (Variables|Default|GetPlayer)) "Collapsed"))))

(event EventWeaponAimExit
  (|CallParentFunction)
  (Utilities|IsValid (stale EventWeaponAimEnter _returnvalue)
    (:Is%20Valid
      (Widget|RemovefromParent (stale EventWeaponAimEnter _returnvalue))
      ;[0 0.02795 0.2656] Weapon, player and HUD visible in game
      (Development|SetHiddeninGame (Variables|Default|GetWeaponMesh) false false)
      (Rendering|SetActorHiddenInGame (Game|GetPlayerCharacter 0) false)
      (Widget|SetVisibility (Variables|/Game/FPSGame/_PlayerCharacter/BP_Player.BP_Player_C|GetMainHUD (Variables|Default|GetPlayer)) "Visible"))))

(event EventStartShooting
  (params (FireType :type E_FireTypes%20Enum :default "NewEnumerator0"))
  (|CallParentFunction FireType)
  (Components|Animation|PlayAnimation (Variables|Default|GetWeaponMesh) "/Game/MilitaryWeaponsSilver/Weapons/Animations/Fire_SniperRifle_W.Fire_SniperRifle_W" false)
  (CallFunction|FireRateCalculate))

(fn ConstructionScript
  (|CallParentFunction))