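; BP_AutoRifle is an automatic rifle weapon that keeps firing from StartShooting until StopShooting.
; It fires immediately, then repeats on a looping timer at the rifle's fire rate.
; Each shot runs the parent weapon's shooting logic and plays the fire animation on the weapon mesh.
; When ammo is empty after a shot, it stops the timer and triggers the player's reload.
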(event Custom|AutoRifleFire
  (if (Variables|Default|GetIsAutoRifleShooting?)
    (|CallParentFunction (stale EventStartShooting FireType))
    (Components|Animation|PlayAnimation (Variables|Default|GetWeaponMesh) "/Game/MilitaryWeapSilver/Weapons/Animations/Fire_Rifle_W.Fire_Rifle_W" false)
    (if (<= (Variables|Default|GetCurrentAmmo) 0)
      (CallFunction|StopShooting)
      (Default|Reload (Variables|Default|GetPlayer)))))

(event EventStopShooting
  (|CallParentFunction)
  (Variables|Default|SetIsAutoRifleShooting? false)
  (Utilities|Time|ClearandInvalidateTimerbyHandle (stale EventStartShooting _returnvalue)))

(event EventStartShooting
  (params (FireType :type E_FireTypes%20Enum :default "NewEnumerator0"))
  (Variables|Default|SetIsAutoRifleShooting? true)
  (CallFunction|AutoRifleFire)
  (bind _returnvalue (Utilities|Time|SetTimerbyEvent (delegate Custom|AutoRifleFire) (Variables|Default|GetAutoRifleFireRate) true)))

(fn ConstructionScript
  (|CallParentFunction))