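; BP_WeaponPickupBase is a base actor for weapon pickups that the player can interact with.
; On BeginPlay it caches the BP_Player, and on interaction it passes its WeaponToSpawn to that player's WeaponPickup.
; A DoOnce then plays the pickup sound and destroys the actor.
; While CanOscillate is set, Tick keeps playing an Oscillate timeline that applies a hover offset to the actor.
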(event Custom|InteractWithWeapon
  ;[0.9534 0.4965 1] Runs event in BP_Player
  (Default|WeaponPickup (Variables|Default|GetPlayer) (Variables|Default|GetWeaponToSpawn))
  (Utilities|FlowControl|DoOnce false
    (:Completed
      (Audio|PlaySound2D (Variables|Default|GetPickUpSound) 1.0 1.0 0.0 0 0)
      (Actor|DestroyActor))))

(event Custom|OscillateWepoan
  (bind _hoveranim (Timeline|Oscillate Play)
    (:Update
      (Transformation|AddActorLocalOffset _hoveranim false false))))

(event EventBeginPlay
  ;[0.9534 0.4965 1] Reference to Player
  (bind _asbp_player (Utilities|Casting|CastToBP_Player (Game|GetPlayerCharacter 0)))
  (Variables|Default|SetPlayer _asbp_player))

(event EventTick
  (params (DeltaSeconds :type Float%20%28single-precision%29))
  (if (Variables|Default|GetCanOscillate?)
    (CallFunction|OscillateWepoan)))

(fn ConstructionScript)