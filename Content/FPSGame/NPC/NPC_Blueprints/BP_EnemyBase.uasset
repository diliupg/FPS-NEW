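; Base enemy NPC character that carries a sword and supplies combat ranges, a patrol route and movement speed tiers.
; On BeginPlay it spawns the sword at the sheath socket and starts LookForLight, a delayed, repeating forward box trace from the head that moves toward a detected player.
; Equip, unequip and attack events play montages, swapping sword sockets on notifies and calling completion dispatchers.
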(event Custom|LookForLight
  (bind _mesh (Variables|Character|GetMesh))
  (bind _returnvalue (Transformation|GetSocketLocation _mesh "HeadSocket"))
  (Utilities|FlowControl|Delay 0.5)
  (bind (_outhit _returnvalue_2) (Collision|BoxTraceByChannel _returnvalue (+ _returnvalue (* (Math|Vector|GetForwardVector (Transformation|GetActorRotation)) 7e+02)) "70.000000,70.000000,50.000000" "0, 0, 0" "TraceTypeQuery1" false 0 "None" true "(R=1.000000,G=0.000000,B=0.000000,A=1.000000)" "(R=0.000000,G=1.000000,B=0.000000,A=1.000000)" 1.0))
  (if _returnvalue_2
    (Utilities|Casting|CastToBP_Player (.HitActor (Collision|BreakHitResult _outhit))
      (:then
        (AI|AIMoveTo self (Transformation|GetWorldLocation (.HitComponent (Collision|BreakHitResult _outhit))) 0 5.0 false
          (:OnSuccess
            _)))
      (:CastFailed
        _)))
  (CallFunction|LookforLight))

(event Custom|SpawnActorAndAttachToSocket
  (Game|SpawnActorfromClass "/Game/FPSGame/WeaponMeshes/Weapons/BP_WeaponBase.BP_WeaponBase_C" (Transformation|GetActorTransform) "Undefined" 0 0)
  (bind _output_get (Variables|Default|SetWeaponActor 0))
  (Transformation|AttachComponentToComponent _output_get (Variables|Character|GetMesh) "SwordSheathSocket" "SnapToTarget" "SnapToTarget" "SnapToTarget" true))

(event Custom|AttackPlayer
  (Animation|Montage|PlayMontage (Variables|Character|GetMesh) "/Game/FPSGame/NPC/EnemyCharacters/EnemyBase/Animations/Montages/Sowrd_Attack_Combo_CL_Heavy_Montage.Sowrd_Attack_Combo_CL_Heavy_Montage"
    (:OnCompleted
      _)
    (:OnInterrupted
      _))
  (Default|CallOnAttackEnd) ; event dispatched only when animation is completed or interrupted.
)

(event EventBeginPlay
  (CallFunction|LookforLight)
  (bind _returnvalue (Game|SpawnActorfromClass "/Game/FPSGame/NPC/EnemyWeapons/BP_WeaponSword.BP_WeaponSword_C" (Transformation|GetActorTransform) "Undefined" 0 0))
  (bind _output_get (Variables|Default|SetWeaponActor _returnvalue))
  (Transformation|AttachComponentToComponent _output_get (Variables|Character|GetMesh) "SwordSheathSocket" "SnapToTarget" "SnapToTarget" "SnapToTarget" true))

(event EventUnEquipWeapon
  (bind _notifyname (Animation|Montage|PlayMontage (Variables|Character|GetMesh) "/Game/FPSGame/NPC/EnemyCharacters/EnemyBase/Animations/Montages/Sword_Sheath_Montage.Sword_Sheath_Montage")
    (:OnCompleted
      (Default|CallOnWeaponUnEquipped))
    (:OnNotifyBegin
      (switch name _notifyname
        (:SheathSword
          (Variables|Default|SetIsWeildingweapon false)
          (Transformation|AttachComponentToComponent (Variables|Default|GetWeaponActor) (Variables|Character|GetMesh) "SwordSheathSocket" "SnapToTarget" "SnapToTarget" "SnapToTarget" true))))))

(event EventEquipWeapon
  (bind _notifyname (Animation|Montage|PlayMontage (Variables|Character|GetMesh) "/Game/FPSGame/NPC/EnemyCharacters/EnemyBase/Animations/Montages/Sword_Weild_Montage.Sword_Weild_Montage")
    (:OnCompleted
      (Default|CallOnWeaponEquipped))
    (:OnNotifyBegin
      (switch name _notifyname
        (:WithdrawSword
          (Transformation|AttachComponentToComponent (Variables|Default|GetWeaponActor) (Variables|Character|GetMesh) "SwordSocket" "SnapToTarget" "SnapToTarget" "SnapToTarget" true)
          (Variables|Default|SetIsWeildingweapon true))))))

(fn ConstructionScript)

(fn GetIdealRange
  (return 1.5e+02 3.5e+02))

(fn GetPatrolRoute
  (return (Variables|Default|GetPatrolRoute)))

(fn SetMovementSpeed
  (params (Speed :type E_MovementSpeed%20Enum :default "NewEnumerator0"))
  (bind _output_get (Variables|/Script/Engine.CharacterMovementComponent|SetMaxWalkSpeed (Variables|Character|GetCharacterMovement) (Utilities|Select :Index Speed :NewEnumerator0 0.0 :NewEnumerator1 2e+02 :NewEnumerator2 3e+02 :NewEnumerator3 5e+02)))
  (return _output_get))