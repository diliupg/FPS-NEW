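; BP_EnemyMelee is a sword-wielding melee enemy that spawns its sword on BeginPlay and attaches it to a sheath socket.
; Equip and unequip events play montages whose notifies move the sword between hand and sheath sockets and set the wielding flag, then signal completion.
; Attack plays a heavy combo montage and signals attack end whether it completes or is interrupted.
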(event EventBeginPlay
  (bind _returnvalue (Game|SpawnActorfromClass "/Game/FPSGame/NPC/EnemyWeapons/BP_WeaponSword.BP_WeaponSword_C" (Transformation|GetActorTransform) "Undefined" 0 0))
  (bind _output_get (Variables|Default|SetWeaponActor _returnvalue))
  (Transformation|AttachComponentToComponent _output_get (Variables|Character|GetMesh) "SwordSheathSocket" "SnapToTarget" "SnapToTarget" "SnapToTarget" true))

(event EventUnEquipWeapon
  (bind _notifyname (Animation|Montage|PlayMontage (Variables|Character|GetMesh) "/Game/FPSGame/NPC/EnemyMeshes/EnemyBase/Animations/Montages/Sword_Sheath_Montage.Sword_Sheath_Montage")
    (:OnCompleted
      (Default|CallOnWeaponUnEquipped))
    (:OnNotifyBegin
      (switch name _notifyname
        (:SheathSword
          (Variables|Default|SetIsWeildingweapon false)
          (Transformation|AttachComponentToComponent (Variables|Default|GetWeaponActor) (Variables|Character|GetMesh) "SwordSheathSocket" "SnapToTarget" "SnapToTarget" "SnapToTarget" true))))))

(event EventEquipWeapon
  (bind _notifyname (Animation|Montage|PlayMontage (Variables|Character|GetMesh) "/Game/FPSGame/NPC/EnemyMeshes/EnemyBase/Animations/Montages/Sword_Weild_Montage.Sword_Weild_Montage")
    (:OnCompleted
      (Default|CallOnWeaponEquipped))
    (:OnNotifyBegin
      (switch name _notifyname
        (:WithdrawSword
          (Transformation|AttachComponentToComponent (Variables|Default|GetWeaponActor) (Variables|Character|GetMesh) "SwordSocket" "SnapToTarget" "SnapToTarget" "SnapToTarget" true)
          (Variables|Default|SetIsWeildingweapon true))))))

(event Collision|EventActorBeginOverlap
  (params (OtherActor :type Actor%20Object%20Reference)))

(event EventTick
  (params (DeltaSeconds :type Float%20%28single-precision%29)))

(event EventAttack
  (Animation|Montage|PlayMontage (Variables|Character|GetMesh) "/Game/FPSGame/NPC/EnemyMeshes/EnemyBase/Animations/Montages/Sowrd_Attack_Combo_CL_Heavy_Montage.Sowrd_Attack_Combo_CL_Heavy_Montage"
    (:OnCompleted
      _)
    (:OnInterrupted
      _))
  (Default|CallOnAttackEnd) ; event dispatched only when animation is completed or interrupted.
)

(fn ConstructionScript
  (|CallParentFunction))