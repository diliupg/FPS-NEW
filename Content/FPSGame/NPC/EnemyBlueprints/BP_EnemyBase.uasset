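; Base enemy character that supplies health, patrol route, combat ranges and movement speeds through getter and setter functions.
; A HealthComponent handles damage and healing; damage responses halt movement, set the AIC_EnemyBase controller to Frozen and play a hit montage.
; Death ragdolls the mesh, stops AI logic and expires body and weapon.
; A delayed, repeating forward box trace from the head sends the enemy toward a detected player.
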(event OnDeath(HealthComponent)
  (Utilities|FlowControl|DoOnce false
    (:Completed
      (Collision|SetCollisionProfileName (Variables|Character|GetMesh) "Ragdoll" true :!class /Script/Engine.PrimitiveComponent)
      (Class|SkeletalMeshComponent|SetAllBodiesSimulatePhysics (Variables|Character|GetMesh) true)
      (AI|Logic|StopLogic (Variables|/Script/AIModule.AIController|GetBrainComponent (Variables|Default|Get%20AIC%20Enemy%20Base)) "")
      (Collision|SetCollisionEnabled (Variables|Collision|GetCapsuleComponent) "NoCollision")
      (Default|SetStateasDead (Variables|Default|Get%20AIC%20Enemy%20Base))
      (Actor|SetLifeSpan 6.0)
      (Actor|SetLifeSpan (Variables|Default|GetWeaponActor) 6.0))))

(event Custom|LookForLight
  (bind _mesh (Variables|Character|GetMesh))
  (bind _returnvalue (Transformation|GetSocketLocation _mesh "HeadSocket"))
  (Utilities|FlowControl|Delay 0.5)
  (bind (_outhit _returnvalue_2) (Collision|BoxTraceByChannel _returnvalue (+ _returnvalue (* (Math|Vector|GetForwardVector (Transformation|GetActorRotation)) 7e+02)) "70.000000,70.000000,50.000000" "0, 0, 0" "TraceTypeQuery1" false 0 "None" true "(R=1.000000,G=0.000000,B=0.000000,A=1.000000)" "(R=0.000000,G=1.000000,B=0.000000,A=1.000000)" 1.0))
  (if _returnvalue_2
    (Utilities|Casting|CastToBP_Player (.HitActor (Collision|BreakHitResult _outhit))
      (:then
        (AI|AIMoveTo self (Transformation|GetWorldLocation (.HitComponent (Collision|BreakHitResult _outhit))) 0 5.0 false
          (:OnSuccess
            _)))
      (:CastFailed
        _)))
  (CallFunction|LookforLight))

(event Custom|PlayHitMontage
  (bind _charactermovement (Variables|Character|GetCharacterMovement))
  (Variables|Default|SettempSpeed (Variables|/Script/Engine.CharacterMovementComponent|GetMaxWalkSpeed _charactermovement))
  (Variables|/Script/Engine.CharacterMovementComponent|SetMaxWalkSpeed _charactermovement 0.0)
  (Animation|PlayAnimMontage "/Game/FPSGame/NPC/EnemyMeshes/EnemyGreen/AnimationsFromMixamo/GreenE_HitReact.GreenE_HitReact" 1.4 (Utilities|String|StringToName (Utilities|String|ToString(Integer) (Math|Random|RandomIntegerinRange 1 2))))
  (Audio|PlaySoundatLocation "/Game/FPSGame/NPC/Audio/Hurt/EnemyHurtSounds.EnemyHurtSounds" (Transformation|GetWorldLocation (Variables|Character|GetMesh)) "0, 0, 0" 1.0 1.0 0.0 0 0 0)
  (Utilities|FlowControl|Delay 0.75)
  (Variables|/Script/Engine.CharacterMovementComponent|SetMaxWalkSpeed _charactermovement (Variables|Default|GettempSpeed)))

(event Custom|HitResponse
  (params (DamageResponse :type E_DamageResponse%20Enum :default "NewEnumerator0"))
  (Components|Movement|StopMovementImmediately (Variables|Character|GetCharacterMovement))
  (Default|SetStateasFrozen (Variables|Default|Get%20AIC%20Enemy%20Base))
  (Animation|Montage|PlayMontage 0 (Variables|Default|GetHitReactMontage)
    (:then
      (Development|PrintString "HitReactBase"))))

(event EventBeginPlay
  (CallFunction|LookforLight)
  (bind _asaic_enemy_base (Utilities|Casting|CastToAIC_EnemyBase (AI|GetAIController self)))
  (Variables|Default|Set%20AIC%20Enemy%20Base _asaic_enemy_base)
  (EventDispatchers|AssignOnDamageResponse (Variables|Default|GetHealthComponent) (EventDispatchers|CreateEvent :!event Custom|HitResponse)))

(fn ConstructionScript
  (bind _healthcomponent (Variables|Default|GetHealthComponent))
  (bind _output_get (Variables|/Game/FPSGame/Blueprints/DamageSystemDG/HealthComponent.HealthComponent_C|SetMaxHealth _healthcomponent 1e+02))
  (Variables|/Game/FPSGame/Blueprints/DamageSystemDG/HealthComponent.HealthComponent_C|SetHealth _healthcomponent _output_get))

(fn GetCurrentHealthBPID
  (return (Variables|/Game/FPSGame/Blueprints/DamageSystemDG/HealthComponent.HealthComponent_C|GetHealth (Variables|Default|GetHealthComponent))))

(fn GetIdealRange
  (return 1.5e+02 3.5e+02))

(fn GetMaxHealthBPID
  (return (Variables|/Game/FPSGame/Blueprints/DamageSystemDG/HealthComponent.HealthComponent_C|GetMaxHealth (Variables|Default|GetHealthComponent))))

(fn GetPatrolRoute
  (return (Variables|Default|GetPatrolRoute)))

(fn HealBPID
  (params (Amount :type Float%20%28single-precision%29))
  (bind _newhealth (Default|Heal (Variables|Default|GetHealthComponent) Amount))
  (return _newhealth))

(fn IsDeadBPID
  (return (Variables|/Game/FPSGame/Blueprints/DamageSystemDG/HealthComponent.HealthComponent_C|GetIsDead (Variables|Default|GetHealthComponent))))

(fn SetMovementSpeed
  (params (Speed :type E_MovementSpeed%20Enum :default "NewEnumerator0"))
  (bind _output_get (Variables|/Script/Engine.CharacterMovementComponent|SetMaxWalkSpeed (Variables|Character|GetCharacterMovement) (Utilities|Select :Index Speed :NewEnumerator0 0.0 :NewEnumerator1 2.5e+02 :NewEnumerator2 4e+02 :NewEnumerator3 5e+02)))
  (return _output_get))

(fn TakeDamageBPID
  (params (DamageInfo :type S%20Damage%20Info%20Structure))
  (bind _wasdamaged (Default|TakeDamageHC (Variables|Default|GetHealthComponent) DamageInfo))
  (return _wasdamaged))